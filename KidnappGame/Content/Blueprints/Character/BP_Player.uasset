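; BP_Player is the player-controlled pawn, handling movement and look input.
; Forward and right axes add movement along the actor's own vectors, scaled by PlayerSpeed, which the IncreaseSpeed action raises while held and lowers on release.
; Horizontal look scales controller yaw by PlayerLookspeed, while vertical look uses a fixed inverted pitch factor that ignores that variable.
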(event Input|ActionEvents|InputActionIncreaseSpeed
  (params (Key :type Key%20Structure :default "None"))
  (:Pressed
    (Variables|Default|SetPlayer_speed 1.0))
  (:Released
    (Variables|Default|SetPlayer_speed 0.5)))

(event Input|AxisEvents|InputAxisMoveForward
  (params (AxisValue :type Float%20%28single-precision%29))
  (Pawn|Input|AddMovementInput (Transformation|GetActorForwardVector) (* AxisValue (Variables|Default|GetPlayer_speed)) false))

(event Input|AxisEvents|InputAxisMoveRight
  (params (AxisValue :type Float%20%28single-precision%29))
  (Pawn|Input|AddMovementInput (Transformation|GetActorRightVector) (* AxisValue (Variables|Default|GetPlayer_speed)) false))

(event Input|AxisEvents|InputAxisLookHorizontal
  (params (AxisValue :type Float%20%28single-precision%29))
  (Pawn|Input|AddControllerYawInput (* AxisValue (Variables|Default|GetPlayer_lookspeed))))

(event Input|AxisEvents|InputAxisLookVertical
  (params (AxisValue :type Float%20%28single-precision%29))
  (Pawn|Input|AddControllerPitchInput (* AxisValue -0.5)))

(fn ConstructionScript)