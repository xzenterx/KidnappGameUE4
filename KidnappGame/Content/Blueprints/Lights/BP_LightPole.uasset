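; BP_LightPole is a light pole with a spot light and an optional flicker effect.
; When the flicker feature is enabled at BeginPlay, a looping retriggerable delay waits a short random interval, then randomly switches the light on or off.
; Each switch sets the spot light intensity and the pole mesh material's illumination parameter together, so the visible lamp glow matches the emitted light.
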(event EventBeginPlay
  (if (Variables|Default|GetFlickerFeature)
    (Utilities|FlowControl|RetriggerableDelay (Math|Random|RandomFloatinRange 0.1 0.2) :!label _label)
    (bind _output_get (Variables|Default|SetFlickerSwitch (Math|Conversions|ToFloat(Integer) (Math|Random|RandomIntegerinRange 0 1))))
    (Rendering|Components|Light|SetIntensity (Variables|Default|GetSpotLight) (* _output_get (Variables|Default|GetLightIntensity)))
    (Rendering|Material|SetScalarParameterValueonMaterials (Variables|Default|GetSM_LightPole_A) "Illum_Intensity" (* (Variables|Default|GetFlickerSwitch) 33.0))
    (goto _label)))

(fn ConstructionScript)